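; CineCamera2D is a visual novel framework camera Blueprint that carries a 2D sprite background for one of four story locations.
; The construction script uses the ENBackground2D enum to select the matching sprite from STBackground2D and applies it to SpriteBackground.
; The choices are Interrogatorio, Crimen, Despacho and CasaMatthew.
; The event graph holds only disabled default events, so it adds no runtime logic.
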(fn `UserConstructionScript`
  (bind (_casamatthew _despacho _crimen _interrogatorio) (break `/Game/VN_Framework/Enums/ST_Background2D` (`self.ST_Background2D`)))
  (`parent.UserConstructionScript`)
  (`PaperSpriteComponent.SetSprite` (`self.Sprite_Background`) (select `/Game/VN_Framework/Enums/EN_Background2D` (`self.EN_Background2D`) :`NewEnumerator0` _interrogatorio :`NewEnumerator1` _crimen :`NewEnumerator2` _despacho :`NewEnumerator3` _casamatthew)))