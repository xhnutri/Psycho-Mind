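; FindCineCamera is a scene-search camera with a magnifier cursor and an object inspection mode.
; Outside inspection, axis inputs pan the camera and zoom its FOV within limits, swapping the cursor widget with zoom state.
; During inspection, zoom slides the object along X, and holding left mouse rotates it by mouse delta; release starts auto-spin.
; Both rotations loop through next-tick timers instead of Tick.
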(event `self.ReceiveBeginPlay`
  (bind _returnvalue (`|CreateWidget` "/Game/Miguel/Widgets/UI/PaC/WD_Lupa.WD_Lupa_C"))
  (`PlayerController.SetMouseCursorWidget` (`GameplayStatics.GetPlayerController` 0) "Default" _returnvalue))

(event `Key|LeftMouseButton`
  (params (Key :type "Key Structure"))
  (:`Pressed`
    (if (`self.Inspection?`)
      (set `self.RotateObject?` false)
      (set `self.RotateObjectByMouse?` true)
      (`self.RotateObjectByMoused`)))
  (:`Released`
    (if (`self.Inspection?`)
      (set `self.RotateObjectByMouse?` false)
      (set `self.RotateObject?` true)
      (`self.RotateObject`))))

(event `RotateObject`
  (bind _returnvalue (* (`GameplayStatics.GetWorldDeltaSeconds`) (`self.SpeedRotate`)))
  (if (`self.RotateObject?`)
    (`KismetSystemLibrary.K2_SetTimerForNextTickDelegate` (delegate `RotateObject`))
    (`SceneComponent.K2_AddWorldRotation` (`self.Object`) (`KismetMathLibrary.MakeRotator` _returnvalue _returnvalue) false false)))

(event `RotateObjectByMoused`
  (bind (_deltax _deltay) (`PlayerController.GetInputMouseDelta` (`GameplayStatics.GetPlayerController` 0)))
  (if (`self.RotateObjectByMouse?`)
    (`KismetSystemLibrary.K2_SetTimerForNextTickDelegate` (delegate `RotateObjectByMoused`))
    (`SceneComponent.K2_AddWorldRotation` (`self.Object`) (* (`KismetMathLibrary.MakeRotator` _deltay 0.0 _deltax) -1.0) false false)))

(event `InputAxis|ZoomObject`
  (params (AxisValue :type "Float (single-precision)"))
  (if (!= AxisValue 0.0)
    (if (`self.Inspection?`)
      (`self.ZoomObjectSelect`)
      (else
        (`self.Zoom Camera Scene`)))))

(event `InputAxis|Horizontal`
  (params (AxisValue :type "Float (single-precision)"))
  (if (not (`self.Inspection?`))
    (`SceneComponent.K2_AddRelativeLocation` (`self.CameraComponent`) (`KismetMathLibrary.MakeVector` 0.0 (* (`self.SpeedMoveCamera`) (`GameplayStatics.GetWorldDeltaSeconds`) AxisValue)) false false)))

(event `InputAxis|Vertical`
  (params (AxisValue :type "Float (single-precision)"))
  (if (not (`self.Inspection?`))
    (`SceneComponent.K2_AddRelativeLocation` (`self.CameraComponent`) (`KismetMathLibrary.MakeVector` 0.0 0.0 (* (`self.SpeedMoveCamera`) (`GameplayStatics.GetWorldDeltaSeconds`) AxisValue)) false false)))

(fn `UserConstructionScript`
  (`parent.UserConstructionScript`))

(fn `Zoom Camera Scene`
  (bind _returnvalue (+ (`CameraComponent.FieldOfView` (`self.CameraComponent`)) (* (`GameplayStatics.GetWorldDeltaSeconds`) (`self.SpeedMoveCamera`) 1.0)))
  (bind _returnvalue_2 (+ (`CameraComponent.FieldOfView` (`self.CameraComponent`)) (* (`GameplayStatics.GetWorldDeltaSeconds`) (`self.SpeedMoveCamera`) -1.0)))
  (if (< (`self.GetInputAxisValue`) 0.0)
    (if (>= _returnvalue (`self.MaxZoomCamera`))
      (`CameraComponent.SetFieldOfView` (`self.CameraComponent`) (`self.MaxZoomCamera`))
      (if (`self.ChangeMouse?`)
        (set `self.ChangeMouse?` false)
        (bind _returnvalue_3 (`|CreateWidget` "/Game/Miguel/Widgets/UI/PaC/WD_Lupa.WD_Lupa_C"))
        (`PlayerController.SetMouseCursorWidget` (`GameplayStatics.GetPlayerController` 0) "Default" _returnvalue_3))
      (else
        (`CameraComponent.SetFieldOfView` (`self.CameraComponent`) _returnvalue)))
    (elif (<= _returnvalue_2 (`self.MinZoomCamera`))
      (`CameraComponent.SetFieldOfView` (`self.CameraComponent`) (`self.MinZoomCamera`))
      (else
        (`CameraComponent.SetFieldOfView` (`self.CameraComponent`) _returnvalue_2)
        (if (not (`self.ChangeMouse?`))
          (set `self.ChangeMouse?` true)
          (bind _returnvalue_4 (`|CreateWidget` "/Game/Miguel/Widgets/UI/PaC/WD_LupaNoZoom.WD_LupaNoZoom_C"))
          (`PlayerController.SetMouseCursorWidget` (`GameplayStatics.GetPlayerController` 0) "Default" _returnvalue_4))))))

(fn `ZoomObjectSelect`
  (bind _x (.x (`SceneComponent.RelativeLocation` (`self.Object`))))
  (if (< (`self.GetInputAxisValue`) 0.0)
    (if (> _x (`self.MinZoomObject`))
      (`SceneComponent.K2_AddRelativeLocation` (`self.Object`) (`KismetMathLibrary.MakeVector` (`self.GetInputAxisValue`)) false false :!label _label))
    (elif (< _x (`self.MaxZoomObject`))
      (goto _label))))