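; BP_Police is a menu actor that simulates a recurring police pass-by with a moving, spinning light and sound.
; After a startup delay, PlayPoliceSound waits, plays a 2D sound and runs a timeline that sets the root's world location.
; The timeline's completion calls the event again, looping the pass indefinitely.
; Tick independently yaws the Police component at LightRotatorSpeed, scaled by delta time.
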(event `self.ReceiveBeginPlay`
  (`KismetSystemLibrary.Delay` 5.0)
  (`self.Play Police Sound`))

(event `Play Police Sound`
  ;[1 1 1] Police Sound
  (`KismetSystemLibrary.Delay` 8.0)
  (`GameplayStatics.PlaySound2D` "/Game/BASTIAN/Sound/Otros/Policia/Policia.Policia" 1.0 1.0 0.0 null null)
  (bind (_direction _police_lights_location) (`Timeline|Timeline_0` :!via `PlayFromStart`)
    (:`Update`
      (`SceneComponent.K2_SetWorldLocation` (`self.DefaultSceneRoot`) _police_lights_location false false))
    (:`Finished`
      (`self.Play Police Sound`))))

(event `self.ReceiveTick`
  (params (DeltaSeconds :type "Float (single-precision)"))
  ;[1 1 1] Police Light Rotator
  (`SceneComponent.K2_AddLocalRotation` (`self.Police`) (* (`KismetMathLibrary.MakeRotator` 0.0 0.0 (`self.Light Rotator Speed`)) DeltaSeconds) false false))

(fn `UserConstructionScript`)