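; BP_SaveGameSettings is a data holder for the menu's saved video settings, covering graphics, shadow, texture and post-process options.
; Each option is stored as a command plus its current selection enum.
; SetSettings writes all of these values at once, while ReturnComands and ReturnEnums read back the commands and the selections separately.
; It only stores values; applying them and writing to disk happen outside these graphs.
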(fn `Return Comands`
  (returns (`Graphic Comand` :type String) (`Shadow Comand` :type String) (`Texture Comand` :type String) (`PostProcess Comand` :type String))
  (return (`self.Graphic Comand`) (`self.Shadow Comand`) (`self.Texture Comand`) (`self.PostProcess Comand`)))

(fn `Return Enums`
  (returns (`Graphic Current` :type "/Game/BASTIAN/0_Menu/Blueprint/SaveMenu/E_Graphic_Settings Enum") (`Post Process Current` :type "/Game/BASTIAN/0_Menu/Blueprint/SaveMenu/E_Graphic_Settings Enum") (`Shadow Current` :type "/Game/BASTIAN/0_Menu/Blueprint/SaveMenu/E_Graphic_Settings Enum") (`Texture Current` :type "/Game/BASTIAN/0_Menu/Blueprint/SaveMenu/E_Graphic_Settings Enum"))
  (return (`self.Graphic Current`) (`self.Post Process Current`) (`self.Shadow Current`) (`self.Texture Current`)))

(fn `Set Settings`
  (params (`Graphic Comand` :type String) (`Shadow Comand` :type String) (`Texture Comand` :type String) (`PostProcess Comand` :type String) (`Graphic Current` :type "/Game/BASTIAN/0_Menu/Blueprint/SaveMenu/E_Graphic_Settings Enum" :default "NewEnumerator0") (`Post Process Current` :type "/Game/BASTIAN/0_Menu/Blueprint/SaveMenu/E_Graphic_Settings Enum" :default "NewEnumerator0") (`Shadow Current` :type "/Game/BASTIAN/0_Menu/Blueprint/SaveMenu/E_Graphic_Settings Enum" :default "NewEnumerator0") (`Texture Current` :type "/Game/BASTIAN/0_Menu/Blueprint/SaveMenu/E_Graphic_Settings Enum" :default "NewEnumerator0"))
  (set `self.Graphic Comand` `Graphic Comand`)
  (set `self.Shadow Comand` `Shadow Comand`)
  (set `self.Texture Comand` `Texture Comand`)
  (set `self.PostProcess Comand` `PostProcess Comand`)
  (set `self.Graphic Current` `Graphic Current`)
  (set `self.Post Process Current` `Post Process Current`)
  (set `self.Shadow Current` `Shadow Current`)
  (set `self.Texture Current` `Texture Current`))