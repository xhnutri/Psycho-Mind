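; Main menu scene Blueprint that fades in the MainMenu widget after a random delay and runs a looping thunderstorm effect behind it.
; The UIOpacity timeline drives the fade, calls StartLightning on every update and shows the mouse cursor when finished.
; StartLightning flickers RectLight with timeline-based random intensity, plays thunder through a DoOnce, then re-triggers after a random delay.
; Matching chains for the other three rect lights are unconnected, so those lights stay hidden.
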(event `self.ReceiveBeginPlay`
  ;[1 1 1] Set light to No visibility
  (`SceneComponent.SetVisibility` (`self.RectLight`) false false)
  (`SceneComponent.SetVisibility` (`self.RectLight1`) false false)
  (`SceneComponent.SetVisibility` (`self.RectLight2`) false false)
  (`SceneComponent.SetVisibility` (`self.RectLight3`) false false)
  (`KismetSystemLibrary.Delay` (`KismetMathLibrary.RandomFloatInRange` 3.5 8.0))
  ;[1 1 1] Main Menu widget
  (bind _returnvalue (`|CreateWidget` "/Game/BASTIAN/0_Menu/Widgets/MainMenu.MainMenu_C"))
  (`UserWidget.AddToViewport` _returnvalue 0)
  (bind (_direction _opacity) (`Timeline|UI Opacity`)
    (:`Update`
      (`Widget.SetRenderOpacity` _returnvalue _opacity)
      (`self.Start Lightning`))
    (:`Finished`
      (set `PlayerController.bShowMouseCursor` true (`GameplayStatics.GetPlayerController` 0)))))

(event `Start Lightning`
  ;[1 1 1] Lightning 1
  (`SceneComponent.SetVisibility` (`self.RectLight`) true false)
  (bind (_direction _intensity) (`Timeline|Lightning Intensity` :!via `PlayFromStart`)
    (:`Update`
      (`LightComponent.SetIntensity` (`self.RectLight`) (`KismetMathLibrary.RandomFloatInRange` (- _intensity 500.0) (+ _intensity 1000.0)))
      (`/Engine/EditorBlueprintResources/StandardMacros.DoOnce` false :!label _label
        (:`Completed`
          (`GameplayStatics.PlaySoundAtLocation` "/Game/BASTIAN/UltraDynamicSky/Sound/Close_Thunder/Close_Thunder_Cue.Close_Thunder_Cue" (`SceneComponent.K2_GetComponentLocation` (`self.RectLight`)) (struct) 1.0 1.0 0.0 null null null null)
          (`KismetSystemLibrary.Delay` 1.0)
          (`SceneComponent.SetVisibility` (`self.RectLight`) false false)
          (`KismetSystemLibrary.Delay` (`KismetMathLibrary.RandomFloatInRange` 3.5 8.0))
          (`self.Start Lightning`)
          (goto _label :!via `Reset`))))))

(fn `UserConstructionScript`)