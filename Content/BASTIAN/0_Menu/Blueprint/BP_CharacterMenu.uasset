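; Menu scene actor that stages the lighting and thunderstorm behind the main menu, and shows the mouse cursor.
; After a short BeginPlay delay, timelines drive the logo and notebook (Libreta) lights while StartLightning begins.
; StartLightning flickers a random rect light via timeline plus random intensity, plays thunder at it, then re-triggers itself after a random pause.
; RandomInteger(3) never selects the fourth lightning branch.
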(event `self.ReceiveBeginPlay`
  ;[1 1 1] Set light to No visibility
  (`SceneComponent.SetVisibility` (`self.RectLight`) false false)
  (`SceneComponent.SetVisibility` (`self.RectLight1`) false false)
  (`SceneComponent.SetVisibility` (`self.RectLight2`) false false)
  (`SceneComponent.SetVisibility` (`self.RectLight3`) false false)
  (`SceneComponent.SetVisibility` (`self.LogoLight`) false false)
  (`SceneComponent.SetVisibility` (`self.LibretaLight`) false false)
  (`KismetSystemLibrary.Delay` 0.7)
  (`|ExecutionSequence`
    (:`then_0`
      (`self.Start Lightning`)
      (set `PlayerController.bShowMouseCursor` true (`GameplayStatics.GetPlayerController` 0)))
    (:`then_1`
      ;[1 1 1] Luces del logo y libreta
      (`SceneComponent.SetVisibility` (`self.LogoLight`) true false)
      (bind (_direction _light) (`Timeline|Timeline_3` :!via `PlayFromStart`)
        (:`Update`
          (`LightComponent.SetIntensity` (`self.LogoLight`) _light))))
    (:`then_2`
      (`SceneComponent.SetVisibility` (`self.LibretaLight`) true false)
      (bind (_direction_2 _light_2) (`Timeline|UI Opacity` :!via `PlayFromStart`)
        (:`Update`
          (`LightComponent.SetIntensity` (`self.LibretaLight`) _light_2))))))

(event `Start Lightning`
  (switch `int` (`KismetMathLibrary.RandomInteger` 3)
    (:`0`
      ;[1 1 1] Lightning 0
      (`SceneComponent.SetVisibility` (`self.RectLight`) true false)
      (bind (_direction _intensity) (`Timeline|Lightning Intensity` :!via `PlayFromStart`)
        (:`Update`
          (`LightComponent.SetIntensity` (`self.RectLight`) (`KismetMathLibrary.RandomFloatInRange` (- _intensity 500.0) (+ _intensity 1000.0)))
          (`/Engine/EditorBlueprintResources/StandardMacros.DoOnce` false :!label _label
            (:`Completed`
              (`GameplayStatics.PlaySoundAtLocation` "/Game/BASTIAN/UltraDynamicSky/Sound/Close_Thunder/Close_Thunder_Cue.Close_Thunder_Cue" (`SceneComponent.K2_GetComponentLocation` (`self.RectLight`)) (struct) 1.0 1.0 0.0 null null null null)
              (`KismetSystemLibrary.Delay` 1.0)
              (`SceneComponent.SetVisibility` (`self.RectLight`) false false)
              (`KismetSystemLibrary.Delay` (`KismetMathLibrary.RandomFloatInRange` 3.5 8.0))
              (`self.Start Lightning`)
              (goto _label :!via `Reset`))))))
    (:`1`
      ;[1 1 1] Lightning 1
      (`SceneComponent.SetVisibility` (`self.RectLight1`) true false)
      (bind (_direction_2 _intensity_2) (`Timeline|Timeline_0` :!via `PlayFromStart`)
        (:`Update`
          (`LightComponent.SetIntensity` (`self.RectLight1`) (`KismetMathLibrary.RandomFloatInRange` (- _intensity_2 500.0) (+ _intensity_2 1000.0)))
          (`/Engine/EditorBlueprintResources/StandardMacros.DoOnce` false :!label _label_2
            (:`Completed`
              (`GameplayStatics.PlaySoundAtLocation` "/Game/BASTIAN/UltraDynamicSky/Sound/Close_Thunder/Close_Thunder_Cue.Close_Thunder_Cue" (`SceneComponent.K2_GetComponentLocation` (`self.RectLight1`)) (struct) 1.0 1.0 0.0 null null null null)
              (`KismetSystemLibrary.Delay` 1.0)
              (`SceneComponent.SetVisibility` (`self.RectLight1`) false false)
              (`KismetSystemLibrary.Delay` (`KismetMathLibrary.RandomFloatInRange` 3.5 8.0))
              (`self.Start Lightning`)
              (goto _label_2 :!via `Reset`))))))
    (:`2`
      ;[1 1 1] Lightning 2
      (`SceneComponent.SetVisibility` (`self.RectLight2`) true false)
      (bind (_direction_3 _intensity_3) (`Timeline|Timeline_1` :!via `PlayFromStart`)
        (:`Update`
          (`LightComponent.SetIntensity` (`self.RectLight2`) (`KismetMathLibrary.RandomFloatInRange` (- _intensity_3 500.0) (+ _intensity_3 1000.0)))
          (`/Engine/EditorBlueprintResources/StandardMacros.DoOnce` false :!label _label_3
            (:`Completed`
              (`GameplayStatics.PlaySoundAtLocation` "/Game/BASTIAN/UltraDynamicSky/Sound/Close_Thunder/Close_Thunder_Cue.Close_Thunder_Cue" (`SceneComponent.K2_GetComponentLocation` (`self.RectLight2`)) (struct) 1.0 1.0 0.0 null null null null)
              (`KismetSystemLibrary.Delay` 1.0)
              (`SceneComponent.SetVisibility` (`self.RectLight2`) false false)
              (`KismetSystemLibrary.Delay` (`KismetMathLibrary.RandomFloatInRange` 3.5 8.0))
              (`self.Start Lightning`)
              (goto _label_3 :!via `Reset`))))))
    (:`3`
      ;[1 1 1] Lightning 3
      (`SceneComponent.SetVisibility` (`self.RectLight3`) true false)
      (bind (_direction_4 _intensity_4) (`Timeline|Timeline_2` :!via `PlayFromStart`)
        (:`Update`
          (`LightComponent.SetIntensity` (`self.RectLight3`) (`KismetMathLibrary.RandomFloatInRange` (- _intensity_4 500.0) (+ _intensity_4 1000.0)))
          (`/Engine/EditorBlueprintResources/StandardMacros.DoOnce` false :!label _label_4
            (:`Completed`
              (`GameplayStatics.PlaySoundAtLocation` "/Game/BASTIAN/UltraDynamicSky/Sound/Close_Thunder/Close_Thunder_Cue.Close_Thunder_Cue" (`SceneComponent.K2_GetComponentLocation` (`self.RectLight3`)) (struct) 1.0 1.0 0.0 null null null null)
              (`KismetSystemLibrary.Delay` 1.0)
              (`SceneComponent.SetVisibility` (`self.RectLight3`) false false)
              (`KismetSystemLibrary.Delay` (`KismetMathLibrary.RandomFloatInRange` 3.5 8.0))
              (`self.Start Lightning`)
              (goto _label_4 :!via `Reset`))))))))

(fn `UserConstructionScript`)