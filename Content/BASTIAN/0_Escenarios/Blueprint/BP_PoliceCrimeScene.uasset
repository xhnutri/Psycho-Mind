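; BP_PoliceCrimeScene is a police crime scene actor that spins a police light.
; Tick rotates the Police component around yaw by LightRotatorSpeed scaled by delta time.
; Delayed siren playback and a timeline that moves the actor's root are disconnected and never run, and PlayPoliceSound is empty.
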(event `self.ReceiveBeginPlay`)

(event `Play Police Sound`
  ;[1 1 1] Police Sound
)

(event `self.ReceiveTick`
  (params (DeltaSeconds :type "Float (single-precision)"))
  ;[1 1 1] Police Light Rotator
  (`SceneComponent.K2_AddLocalRotation` (`self.Police`) (* (`KismetMathLibrary.MakeRotator` 0.0 0.0 (`self.Light Rotator Speed`)) DeltaSeconds) false false))

(fn `UserConstructionScript`)