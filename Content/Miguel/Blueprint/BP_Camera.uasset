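; BP_Camera spins its Cube component around world roll and pitch at a frame-rate-scaled SpeedRotate while the RotateObject flag is set.
; The RotateObject event starts on BeginPlay and loops by rescheduling itself for the next tick, leaving Event Tick empty.
; Holding left mouse clears the flag to stop the loop, and releasing restarts it.
; Key 0 only prints a message, and leftover timer-debug nodes are unwired.
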(event `self.ReceiveBeginPlay`
  (`self.RotateObject`))

(event `self.ReceiveTick`
  (params (DeltaSeconds :type "Float (single-precision)")))

(event `RotateObject`
  (bind _returnvalue (* (`GameplayStatics.GetWorldDeltaSeconds`) (`self.SpeedRotate`)))
  (if (`self.RotateObject?`)
    (`KismetSystemLibrary.K2_SetTimerForNextTickDelegate` (delegate `RotateObject`))
    (`SceneComponent.K2_AddWorldRotation` (`self.Cube`) (`KismetMathLibrary.MakeRotator` _returnvalue _returnvalue) false false)))

(event `Key|Zero`
  (params (Key :type "Key Structure"))
  (:`Pressed`
    (`KismetSystemLibrary.PrintString` "False Rotate")))

(event `Key|LeftMouseButton`
  (params (Key :type "Key Structure"))
  (:`Pressed`
    (set `self.RotateObject?` false)
    (`KismetSystemLibrary.PrintString` "Presend"))
  (:`Released`
    (set `self.RotateObject?` true)
    (`self.RotateObject`)
    (`KismetSystemLibrary.PrintString` "Released")))

(fn `UserConstructionScript`)