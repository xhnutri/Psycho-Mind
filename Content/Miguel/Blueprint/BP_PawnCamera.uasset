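; Camera pawn for viewing a scene and inspecting objects, with a magnifier-style cursor widget.
; InitObject copies a mesh and material onto the Object component and enters inspection, where it auto-rotates via next-tick timers until left-mouse drag rotates it.
; The zoom axis moves the object within limits during inspection; otherwise it changes camera FOV and swaps the cursor widget.
; Outside inspection, Horizontal and Vertical axes pan the camera.
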(event `InitObject`
  (params (NewObject :type "StaticMeshComponent Object Reference"))
  (bind _object (`self.Object`))
  (set `self.Inspection?` true)
  (`PrimitiveComponent.SetMaterial` _object 0 (`PrimitiveComponent.GetMaterial` NewObject 0))
  (`StaticMeshComponent.SetStaticMesh` _object (`StaticMeshComponent.StaticMesh` NewObject))
  (`SceneComponent.SetVisibility` (`self.Object`) true false)
  (`self.RotateObject`))

(event `self.ReceiveBeginPlay`
  (bind _returnvalue (`|CreateWidget` "/Game/Miguel/Widgets/UI/PaC/WD_Lupa.WD_Lupa_C"))
  (`PlayerController.SetMouseCursorWidget` (`GameplayStatics.GetPlayerController` 0) "Default" _returnvalue))

(event `Key|LeftMouseButton`
  (params (Key :type "Key Structure"))
  (:`Pressed`
    (if (`self.Inspection?`)
      (set `self.RotateObject?` false)
      (set `self.RotateObjectByMouse?` true)
      (`self.RotateObjectByMouse`)))
  (:`Released`
    (if (`self.Inspection?`)
      (set `self.RotateObjectByMouse?` false)
      (set `self.RotateObject?` true)
      (`self.RotateObject`))))

(event `RotateObject`
  (bind _returnvalue (* (`GameplayStatics.GetWorldDeltaSeconds`) (`self.SpeedRotate`)))
  (if (`self.RotateObject?`)
    (`KismetSystemLibrary.K2_SetTimerForNextTickDelegate` (delegate `RotateObject`))
    (`SceneComponent.K2_AddWorldRotation` (`self.Object`) (`KismetMathLibrary.MakeRotator` _returnvalue _returnvalue) false false)))

(event `RotateObjectByMouse`
  (bind (_deltax _deltay) (`PlayerController.GetInputMouseDelta` (`GameplayStatics.GetPlayerController` 0)))
  (if (`self.RotateObjectByMouse?`)
    (`KismetSystemLibrary.K2_SetTimerForNextTickDelegate` (delegate `RotateObjectByMouse`))
    (`SceneComponent.K2_AddWorldRotation` (`self.Object`) (* (`KismetMathLibrary.MakeRotator` _deltay 0.0 _deltax) -1.0) false false)))

(event `InputAxis|ZoomObject`
  (params (AxisValue :type "Float (single-precision)"))
  (if (!= AxisValue 0.0)
    (if (`self.Inspection?`)
      (`self.ZoomObjectSelect`)
      (else
        (`self.Zoom Camera Scene`)))))

(event `InputAxis|Horizontal`
  (params (AxisValue :type "Float (single-precision)"))
  (if (not (`self.Inspection?`))
    (`SceneComponent.K2_AddRelativeLocation` (`self.Camera`) (`KismetMathLibrary.MakeVector` 0.0 (* (`self.SpeedMoveCamera`) (`GameplayStatics.GetWorldDeltaSeconds`) AxisValue)) false false)))

(event `InputAxis|Vertical`
  (params (AxisValue :type "Float (single-precision)"))
  (if (not (`self.Inspection?`))
    (`SceneComponent.K2_AddRelativeLocation` (`self.Camera`) (`KismetMathLibrary.MakeVector` 0.0 0.0 (* (`self.SpeedMoveCamera`) (`GameplayStatics.GetWorldDeltaSeconds`) AxisValue)) false false)))

(fn `UserConstructionScript`)

(fn `Zoom Camera Scene`
  (bind _returnvalue (+ (`CameraComponent.FieldOfView` (`self.Camera`)) (* (`GameplayStatics.GetWorldDeltaSeconds`) (`self.SpeedMoveCamera`) 1.0)))
  (bind _returnvalue_2 (+ (`CameraComponent.FieldOfView` (`self.Camera`)) (* (`GameplayStatics.GetWorldDeltaSeconds`) (`self.SpeedMoveCamera`) -1.0)))
  (if (< (`self.GetInputAxisValue`) 0.0)
    (if (>= _returnvalue (`self.MaxZoomCamera`))
      (`CameraComponent.SetFieldOfView` (`self.Camera`) (`self.MaxZoomCamera`))
      (if (`self.ChangeMouse?`)
        (set `self.ChangeMouse?` false)
        (bind _returnvalue_3 (`|CreateWidget` "/Game/Miguel/Widgets/UI/PaC/WD_Lupa.WD_Lupa_C"))
        (`PlayerController.SetMouseCursorWidget` (`GameplayStatics.GetPlayerController` 0) "Default" _returnvalue_3))
      (else
        (`CameraComponent.SetFieldOfView` (`self.Camera`) _returnvalue)))
    (elif (<= _returnvalue_2 (`self.MinZoomCamera`))
      (`CameraComponent.SetFieldOfView` (`self.Camera`) (`self.MinZoomCamera`))
      (else
        (`CameraComponent.SetFieldOfView` (`self.Camera`) _returnvalue_2)
        (if (not (`self.ChangeMouse?`))
          (set `self.ChangeMouse?` true)
          (bind _returnvalue_4 (`|CreateWidget` "/Game/Miguel/Widgets/UI/PaC/WD_LupaNoZoom.WD_LupaNoZoom_C"))
          (`PlayerController.SetMouseCursorWidget` (`GameplayStatics.GetPlayerController` 0) "Default" _returnvalue_4))))))

(fn `ZoomObjectSelect`
  (bind _x (.x (`SceneComponent.RelativeLocation` (`self.Object`))))
  (if (< (`self.GetInputAxisValue`) 0.0)
    (if (> _x (`self.MinZoomObject`))
      (`SceneComponent.K2_AddRelativeLocation` (`self.Object`) (`KismetMathLibrary.MakeVector` (`self.GetInputAxisValue`)) false false :!label _label))
    (elif (< _x (`self.MaxZoomObject`))
      (goto _label))))