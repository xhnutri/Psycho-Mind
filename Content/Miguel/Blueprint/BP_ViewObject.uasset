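; BP_ViewObject is a clickable world object that hands its Cube mesh to the BP_PawnCamera pawn.
; On BeginPlay it enables the mouse cursor with click and hover events.
; Hovering the Cube switches to a grab-hand cursor, shows a text label and raises the material's emissive multiplier.
; Clicking calls InitObject on the player's camera pawn with the Cube and hides the Scene component.
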(event `self.ReceiveBeginPlay`
  (bind _returnvalue (`GameplayStatics.GetPlayerController` 0))
  (set `PlayerController.bEnableMouseOverEvents` true _returnvalue)
  (set `PlayerController.bShowMouseCursor` true _returnvalue)
  (set `PlayerController.bEnableClickEvents` true _returnvalue))

(event `self.Cube.OnBeginCursorOver`
  (params (TouchedComponent :type "PrimitiveComponent Object Reference"))
  (set `PlayerController.CurrentMouseCursor` "GrabHand" (`GameplayStatics.GetPlayerController` 0))
  (`SceneComponent.SetVisibility` (`self.TextRender`) true false)
  (`MeshComponent.SetScalarParameterValueOnMaterials` (`self.Cube`) "EmissiveMultiplier" 10.0)
  (`KismetSystemLibrary.PrintString` "Hello"))

(event `self.Cube.OnEndCursorOver`
  (params (TouchedComponent :type "PrimitiveComponent Object Reference"))
  (set `PlayerController.CurrentMouseCursor` "Default" (`GameplayStatics.GetPlayerController` 0))
  (`SceneComponent.SetVisibility` (`self.TextRender`) false false)
  (`MeshComponent.SetScalarParameterValueOnMaterials` (`self.Cube`) "EmissiveMultiplier" 0.0))

(event `self.Cube.OnClicked`
  (params (TouchedComponent :type "PrimitiveComponent Object Reference") (ButtonPressed :type "Key Structure"))
  (bind _asbp_pawn_camera (cast `/Game/Miguel/Blueprint/BP_PawnCamera` (`GameplayStatics.GetPlayerPawn` 0)))
  (`/Game/Miguel/Blueprint/BP_PawnCamera.InitObject` _asbp_pawn_camera (`self.Cube`))
  (`SceneComponent.SetVisibility` (`self.Scene`) false false))

(fn `UserConstructionScript`)