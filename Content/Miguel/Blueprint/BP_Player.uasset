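; Player Blueprint that drives a dialogue scene widget fed from the DT_Scene1 data table.
; On BeginPlay it creates W_DialogueScene, adds it to the viewport, blocking-loads the table and appends each row's SpecialEvent as text to the widget's DTRichText array.
; Pressing the 0 key calls WriteText on the widget and prints a debug message.
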(event `self.ReceiveBeginPlay`
  (`|ExecutionSequence`
    (:`then_1`
      (bind _returnvalue (`|CreateWidget` "/Game/Miguel/Widgets/W_DialogueScene.W_DialogueScene_C"))
      (bind _output_get (set `self.W_Scene1` _returnvalue))
      (`UserWidget.AddToViewport` _output_get 0)
      (bind _returnvalue_2 (`KismetSystemLibrary.LoadAsset_Blocking` "/Game/Miguel/DataTable/DT_Scene1.DT_Scene1"))
      (bind _asdata_table (cast `DataTable` _returnvalue_2))
      (bind _outrownames (`DataTableFunctionLibrary.GetDataTableRowNames` _asdata_table))
      (for _array_element _outrownames
        (bind _returnvalue_3 (`|GetDataTableRow` _asdata_table _array_element)
          (:`then`
            (`KismetArrayLibrary.Array_Add` (`/Game/Miguel/Widgets/W_DialogueScene.DT_RichText` (`self.W_Scene1`)) (`KismetTextLibrary.Conv_StringToText` (`.SpecialEvent_13_21C370D249976663DBDC13835EB465DD` (break `/Game/Miguel/Structures/ST_DialogueScene` _returnvalue_3)))))
          (:`RowNotFound`
            (`KismetSystemLibrary.PrintString` "Not ffound")))))))

(event `Key|Zero`
  (params (Key :type "Key Structure"))
  (:`Pressed`
    (`/Game/Miguel/Widgets/W_DialogueScene.WriteText` (`self.W_Scene1`))
    (`KismetSystemLibrary.PrintString` "Click")))

(fn `UserConstructionScript`)