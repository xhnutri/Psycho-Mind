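; Visual novel dialogue controller that plays data-table scenes with a typewriter effect, registering itself on the player pawn.
; StartScene async-loads scene lines and character info, spawns WB_Dialogue2D and sets page and background.
; A delayed dispatcher loop reveals text in random steps with key sounds, wrapping underlined phrases in rich-text tags.
; NextTextWriter completes the current line or advances, updating speaker sprite and colors, then chains to the next scene.
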(event `self.ReceiveBeginPlay`
  (set `PlayerController.bShowMouseCursor` true (`GameplayStatics.GetPlayerController` 0))
  (bind _asbp_pmpawn_player (cast `/Game/NewVN_Framework/BP_PMPawnPlayer` (`GameplayStatics.GetPlayerPawn` 0)))
  (set `/Game/NewVN_Framework/BP_PMPawnPlayer.BP_TypeWrite` self _asbp_pmpawn_player)
  (set `self.PawnController` _asbp_pmpawn_player))

(event `InitScene`
  (params (Scene :type Name))
  (bind _object (`|LoadAsset` "/Game/NewVN_Framework/TableData/MainScene/DT_MainScenes.DT_MainScenes")
    (:`Completed`
      (bind _asdata_table (cast `DataTable` _object))
      (bind _returnvalue (`|GetDataTableRow` _asdata_table Scene)
        (:`then`
          (bind _output_get (set `self.ST_MainScenes` _returnvalue))
          (bind ((`Datatable_5_289E267A487BDBC2951F05A10643630C` _datatable)) (break `/Game/NewVN_Framework/TableData/MainScene/ST_MainScenes` _output_get))
          (bind _outrownames (`DataTableFunctionLibrary.GetDataTableRowNames` _datatable))
          (for _array_element _outrownames
            (bind _returnvalue_2 (`|GetDataTableRow` _datatable _array_element)
              (:`then`
                (`KismetArrayLibrary.Array_Add` (`self.ST_TableScenesText`) _returnvalue_2))))
          (bind _object_2 (`|LoadAsset` "/Game/NewVN_Framework/TableData/Character/DT_Characters.DT_Characters")
            (:`Completed`
              (bind _asdata_table_2 (cast `DataTable` _object_2))
              (bind _outrownames_2 (`DataTableFunctionLibrary.GetDataTableRowNames` _asdata_table_2))
              (for _array_element_2 _outrownames_2
                (bind _returnvalue_3 (`|GetDataTableRow` _asdata_table_2 _array_element_2)
                  (:`then`
                    (for _array_element_3 (`.CharactersScene_53_A0212D58467AD36D502C288531CF1BA7` (break `/Game/NewVN_Framework/TableData/MainScene/ST_MainScenes` (`self.ST_MainScenes`)))
                      (if (`|EnumEquality` _array_element_3 (`.Character_52_81CE848D46DF432F314589B433504745` (break `/Game/NewVN_Framework/TableData/Character/ST_TableCharacter` _returnvalue_3)))
                        (`BlueprintMapLibrary.Map_Add` (`self.ST_FindCharacterInfo`) _array_element_3 _returnvalue_3)
                        (break))))))
              (`self.InitSceneValues`))))
        (:`RowNotFound`
          (`KismetSystemLibrary.PrintString` "Could Not Found Scene"))))))

(event `InitSceneValues`
  (`self.ExitsScene`
    (:`Exits`
      (`self.SpawnWBDialogue2D`)
      (`self.SetValuesScene`)
      (`self.BeginPlayTypeWrite`))))

(event `BeginPlayTypeWrite`
  (add `self.DisTextWriter` (delegate `TextWriterAnim`))
  (`KismetSystemLibrary.Delay` 0.7)
  (`self.GetSceneText`))

(event `TextWriterAnim`
  (bind _complete (`self.TextWriteLength` (`KismetStringLibrary.Len` (`.Text_8_2695685D4E022C26AB8B52BA1EFE8666` (break `/Game/NewVN_Framework/TableData/Scenes/ST_SceneText` (`self.ST_SceneText`))))))
  (if _complete
    (bind _textunderline (`self.GetTextUnderline` (`self.TextWriteIndex`)))
    (`/Game/NewVN_Framework/Widgets/WB_Dialogue2D.ChangeText` (`self.WBDialogue2D`) _textunderline)
    (bind (_st_tablecharacters _exits) (`self.GetCharacter`))
    (`self.ExitsValue` _exits
      (:`Exits`
        (`GameplayStatics.PlaySound2D` (`.KeySound_51_1A1DB43D4377630DF8F838BCC035ED2A` (break `/Game/NewVN_Framework/TableData/Character/ST_TableCharacter` _st_tablecharacters)) 1.0 1.0 0.0 null null))
      (:`Not Exits`
        _))
    (`KismetSystemLibrary.Delay` (`KismetMathLibrary.RandomFloatInRange` 0.04 0.06))
    (`self.DisTextWriter`)
    (else
      (set `self.TextWriteIndex` 0)
      (set `self.InitTextWriter?` false))))

(event `NextTextWriter`
  (if (`self.InitTextWriter?`)
    (clear `self.DisTextWriter`)
    (bind _textunderline (`self.GetTextUnderline` (`KismetStringLibrary.Len` (`.Text_8_2695685D4E022C26AB8B52BA1EFE8666` (break `/Game/NewVN_Framework/TableData/Scenes/ST_SceneText` (`self.ST_SceneText`))))))
    (`/Game/NewVN_Framework/Widgets/WB_Dialogue2D.ChangeText` (`self.WBDialogue2D`) _textunderline)
    (set `self.InitTextWriter?` false)
    (set `self.TextWriteIndex` 0)
    (else
      (`/Engine/EditorBlueprintResources/StandardMacros.IncrementInt` (`self.TextSceneIndex`)
        (:`  `
          (`self.ExitsScene`
            (:`Exits`
              (add `self.DisTextWriter` (`|CreateDelegate` :!event `TextWriterAnim`))
              (`self.GetSceneText`))
            (:`Not Exits`
              (clear `self.DisNextScene`)
              (`self.NextScene`))))))))

(fn `GetCharacter`
  (returns (ST_TableCharacters :type "/Game/NewVN_Framework/TableData/Character/ST_TableCharacter Structure") (Exits :type Boolean))
  (bind (_value _returnvalue) (`BlueprintMapLibrary.Map_Find` (`self.ST_FindCharacterInfo`) (`.Character_6_EE776487462751F5329E498891714F85` (break `/Game/NewVN_Framework/TableData/Scenes/ST_SceneText` (`self.ST_SceneText`)))))
  (return _value _returnvalue))

(fn `GetSceneText`
  (set `self.InitTextWriter?` true)
  (add `self.DisNextScene` (`|CreateDelegate` :!event `NextTextWriter`))
  (`self.SetValuesSceneText`)
  (`self.DisTextWriter`))

(fn `GetTextUnderline`
  (params (TextWrite :type Integer))
  (returns (TextUnderline :type String))
  (locals (Text :type String) (IndexText :type Integer) (TextPosition :type "/Game/NewVN_Framework/Structures/ST_TextUnderline Structure") (ArrayIndex :type Integer))
  (bind ((`Index_8_56428A2C490E4A84B08223B0DADAEE3B` _index) (`LastIndex_6_8BF9328242DFB21168867B9670A744D7` _lastindex)) (break `/Game/NewVN_Framework/Structures/ST_TextUnderline` (`local.TextPosition`)))
  (bind ((`Index_8_56428A2C490E4A84B08223B0DADAEE3B` _index_2)) (break `/Game/NewVN_Framework/Structures/ST_TextUnderline` (`local.TextPosition`)))
  (bind ((`LastIndex_6_8BF9328242DFB21168867B9670A744D7` _lastindex_2)) (break `/Game/NewVN_Framework/Structures/ST_TextUnderline` (`local.TextPosition`)))
  (bind ((`Index_8_56428A2C490E4A84B08223B0DADAEE3B` _index_3) (`Length_7_6756AFD94F4A1A637D3B5BA23D88250E` _length)) (break `/Game/NewVN_Framework/Structures/ST_TextUnderline` (`local.TextPosition`)))
  (set `local.IndexText` TextWrite)
  (set `local.Text` (`.Text_8_2695685D4E022C26AB8B52BA1EFE8666` (break `/Game/NewVN_Framework/TableData/Scenes/ST_SceneText` (`self.ST_SceneText`))))
  (if (> (`KismetArrayLibrary.Array_Length` (`self.ArrayTextUnderline`)) 0)
    (for (_array_element _array_index) (`self.ArrayTextUnderline`)
      (set `local.TextPosition` _array_element)
      (set `local.ArrayIndex` _array_index)
      (if (>= (`KismetStringLibrary.Len` (`KismetStringLibrary.GetSubstring` (`local.Text`) 0 (`local.IndexText`))) _index)
        (if (< (`local.IndexText`) _lastindex)
          (set `local.Text` (`KismetStringLibrary.Concat_StrStr` (`KismetStringLibrary.GetSubstring` (`local.Text`) 0 _index_2) "<" (`.UnderlineTextNameTable_22_0A866E5341C36B0B3CF051AEA389F63E` (break `/Game/NewVN_Framework/TableData/Scenes/ST_SceneText` (`self.ST_SceneText`))) ">" (`KismetStringLibrary.GetSubstring` (`local.Text`) _index_2 (- (`local.IndexText`) _index_2)) "</>"))
          (else
            (set `local.Text` (`KismetStringLibrary.Concat_StrStr` (`KismetStringLibrary.GetSubstring` (`local.Text`) 0 _index_3) "<" (`.UnderlineTextNameTable_22_0A866E5341C36B0B3CF051AEA389F63E` (break `/Game/NewVN_Framework/TableData/Scenes/ST_SceneText` (`self.ST_SceneText`))) ">" (`KismetStringLibrary.GetSubstring` (`local.Text`) _index_3 _length) "</>" (`KismetStringLibrary.GetSubstring` (`local.Text`) _lastindex_2 (- (`local.IndexText`) _lastindex_2))))))
        (set `local.IndexText` (+ (`local.IndexText`) (+ (`KismetStringLibrary.Len` (`.UnderlineTextNameTable_22_0A866E5341C36B0B3CF051AEA389F63E` (break `/Game/NewVN_Framework/TableData/Scenes/ST_SceneText` (`self.ST_SceneText`)))) 5)))
        (elif (> (`local.ArrayIndex`) 0)
          (return (`local.Text`))
          (else
            (return (`KismetStringLibrary.GetSubstring` (`local.Text`) 0 (`local.IndexText`)))))))
    (return (`local.Text`))
    (else
      (return (`KismetStringLibrary.GetSubstring` (`local.Text`) 0 (`local.IndexText`))))))

(fn `NextScene`
  (bind (_datatable _nextscene) (break `/Game/NewVN_Framework/TableData/MainScene/ST_MainScenes` (`self.ST_MainScenes`)))
  (if (`|EnumInequality` _nextscene "NewEnumerator14")
    (`self.StartScene` _nextscene)))

(fn `SetValuesScene`
  (bind ((`Page_42_D1849EB64C9530F7F4EB8888FC5AEDB6` _page) (`Background2D_48_D66C7D6C4A47F4ED40E0A499AE6DB5FB` _background2d)) (break `/Game/NewVN_Framework/TableData/MainScene/ST_MainScenes` (`self.ST_MainScenes`)))
  (`/Game/NewVN_Framework/Widgets/WB_Dialogue2D.ChangePage` (`self.WBDialogue2D`) _page)
  (`/Game/NewVN_Framework/BP_PMPawnPlayer.ChangeBackground` (`self.PawnController`) _background2d))

(fn `SetValuesSceneText`
  (bind ((`Character_6_EE776487462751F5329E498891714F85` _character) (`TextColor_19_98C54B2E4F02375FE0A79FB6FFE68910` _textcolor)) (break `/Game/NewVN_Framework/TableData/Scenes/ST_SceneText` (`self.ST_SceneText`)))
  (set `self.ST_SceneText` (`|GetArrayItem` (`self.ST_TableScenesText`) (`self.TextSceneIndex`)))
  (`/Game/NewVN_Framework/Widgets/WB_Dialogue2D.ChangeCharacter` (`self.WBDialogue2D`) _character)
  (`/Game/NewVN_Framework/Widgets/WB_Dialogue2D.ChangeTextColor` (`self.WBDialogue2D`) _textcolor)
  (`self.TextUnderline`)
  (bind (_st_tablecharacters _exits) (`self.GetCharacter`))
  (`self.ExitsValue` _exits
    (:`Exits`
      (bind ((`Character_52_81CE848D46DF432F314589B433504745` _character_2) (`NameColor_53_E29CC765409EF906F225A6BD3F4849C9` _namecolor) (`Sprite_56_F2BCCBFE417E05058AC076B6D20E3252` _sprite)) (break `/Game/NewVN_Framework/TableData/Character/ST_TableCharacter` _st_tablecharacters))
      (`/Game/NewVN_Framework/Widgets/WB_Dialogue2D.ChangeColorCharacter` (`self.WBDialogue2D`) _namecolor)
      (`/Game/NewVN_Framework/BP_PMPawnPlayer.ChangeSpriteCharacter` (`self.PawnController`) _sprite _character_2))))

(fn `SpawnWBDialogue2D`
  (bind _foundwidgets (`WidgetBlueprintLibrary.GetAllWidgetsOfClass` "/Game/NewVN_Framework/Widgets/WB_Dialogue2D.WB_Dialogue2D_C"))
  (for _array_element _foundwidgets
    (`Widget.RemoveFromParent` _array_element))
  (bind _returnvalue (`|CreateWidget` "/Game/NewVN_Framework/Widgets/WB_Dialogue2D.WB_Dialogue2D_C"))
  (set `self.WBDialogue2D` _returnvalue)
  (`UserWidget.AddToViewport` (`self.WBDialogue2D`) 0))

(fn `StartScene`
  (params (Scene :type "/Game/NewVN_Framework/Enums/EN_ScenesPM Enum" :default "NewEnumerator14"))
  (`self.InitScene` (`KismetStringLibrary.Conv_StringToName` (`|GetEnumeratorNameAsString` Scene))))

(fn `TextUnderline`
  (locals (LenText :type Integer) (ArrayText :type "Array of /Game/NewVN_Framework/Structures/ST_TextUnderline Structure"))
  (bind ((`Text_8_2695685D4E022C26AB8B52BA1EFE8666` _text) (`UnderlineText_18_04F867734D1396FBB7A903B0B2970186` _underlinetext)) (break `/Game/NewVN_Framework/TableData/Scenes/ST_SceneText` (`self.ST_SceneText`)))
  (`KismetArrayLibrary.Array_Clear` (`self.ArrayTextUnderline`))
  (for _array_element _underlinetext
    (bind _returnvalue (`KismetStringLibrary.FindSubstring` _text _array_element))
    (bind _returnvalue_2 (+ (`local.LenText`) _returnvalue))
    (bind _returnvalue_3 (+ _returnvalue (`KismetStringLibrary.Len` _array_element) (`local.LenText`)))
    (`KismetArrayLibrary.Array_Add` (`self.ArrayTextUnderline`) (make `/Game/NewVN_Framework/Structures/ST_TextUnderline` _returnvalue_2 _returnvalue_3 (- _returnvalue_3 _returnvalue_2)))
    (set `local.LenText` (+ (`KismetStringLibrary.Len` (`.UnderlineTextNameTable_22_0A866E5341C36B0B3CF051AEA389F63E` (break `/Game/NewVN_Framework/TableData/Scenes/ST_SceneText` (`self.ST_SceneText`)))) 5))))

(fn `TextWriteLength`
  (params (Len :type Integer))
  (returns (Complete :type Boolean))
  (bind _textwriteindex (`self.TextWriteIndex`))
  (if (< (`self.TextWriteIndex`) (`local.Len`))
    (if (>= (`self.TextWriteIndex`) (`local.Len`))
      (set `self.TextWriteIndex` (`local.Len`))
      (else
        (set `self.TextWriteIndex` (`KismetMathLibrary.RandomIntegerInRange` _textwriteindex (+ _textwriteindex 4)))))
    (return true)
    (else
      (return false))))

(fn `UserConstructionScript`)