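; Point-and-click player for inspecting a 2D crime scene for clues.
; Tick traces under the mouse, swapping the scene sprite to the hovered clue's and toggling magnifier cursor widgets.
; Zoom scales scene and clue sprites rather than moving the lens, adjusting the limits for axis-driven camera panning.
; Clicking the S_Pedant clue reveals a 3D object that auto-spins or follows mouse drag through self-rescheduling next-tick timers.
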(event `ChangeSizeSprite`
  (`KismetSystemLibrary.K2_SetTimerForNextTickDelegate` (delegate `ChangeSizeSprite`)))

(event `self.ReceiveBeginPlay`
  (bind _returnvalue (`GameplayStatics.GetPlayerController` 0))
  (`self.MouseLupaNoZoom`)
  (set `self.InitSprite` (`PaperSpriteComponent.GetSprite` (`self.S_SceneCrimen_2`)))
  (set `PlayerController.bShowMouseCursor` true _returnvalue)
  (set `PlayerController.bEnableMouseOverEvents` true _returnvalue)
  (set `PlayerController.bEnableClickEvents` true _returnvalue))

(event `self.ReceiveTick`
  (params (DeltaSeconds :type "Float (single-precision)"))
  (bind (_worldlocation _worlddirection) (`PlayerController.DeprojectMousePositionToWorld` (`GameplayStatics.GetPlayerController` 0)))
  (`|ExecutionSequence`
    (:`then_0`
      (bind (_outhit _returnvalue) (`KismetSystemLibrary.LineTraceSingle` _worldlocation (+ _worldlocation (* _worlddirection 10000)) "TraceTypeQuery1"))
      (if _returnvalue
        (bind _aspaper_sprite_actor (cast `PaperSpriteActor` (`.HitActor` (`GameplayStatics.BreakHitResult` _outhit)))
          (:`then`
            (bind _returnvalue_2 (`PaperSpriteComponent.GetSprite` (`PaperSpriteActor.RenderComponent` _aspaper_sprite_actor)))
            (`PaperSpriteComponent.SetSprite` (`self.S_SceneCrimen_2`) _returnvalue_2)
            (if (not (`self.ViewObject?`))
              (set `self.ViewObject?` true)
              (set `self.NamePista` (`KismetSystemLibrary.GetObjectName` _returnvalue_2))
              (`self.MouseLupaZoom`)))
          (:`CastFailed`
            (`PaperSpriteComponent.SetSprite` (`self.S_SceneCrimen_2`) (`self.InitSprite`) :!label _label)
            (if (`self.ViewObject?`)
              (set `self.ViewObject?` false)
              (`self.MouseLupaNoZoom`))))
        (else
          (goto _label))))))

(event `InputAxis|ZoomObject`
  (params (AxisValue :type "Float (single-precision)"))
  (if (!= (`self.GetInputAxisValue`) 0.0)
    (if (and (== (`self.GetInputAxisValue`) 0.0) (== (`self.GetInputAxisValue`) 0.0))
      (set `self.DelayZoom?` true)
      (set `self.Zoom?` true)
      (`self.ZoomBySpriteNew` (`self.GetScaleAdd`)))
    (elif (`self.Zoom?`)
      (`KismetSystemLibrary.Delay` 0.2)
      (set `self.DelayZoom?` false))))

(event `InputAxis|Horizontal`
  (params (AxisValue :type "Float (single-precision)"))
  (if (not (`self.DelayZoom?`))
    (`self.MoveHorizontalAxis` AxisValue (`self.MaxHorizontal`))))

(event `InputAxis|Vertical`
  (params (AxisValue :type "Float (single-precision)"))
  (if (not (`self.DelayZoom?`))
    (`self.MoveVerticalAxis` AxisValue (`self.MaxVertical`))))

(event `InputAction|Click`
  (params (Key :type "Key Structure"))
  (:`Pressed`
    (if (`self.Inspection?`)
      _
      (elif (`self.RotateObject?`)
        (set `self.RotateObject?` false)
        (set `self.RotateObjectByMouse?` true)
        (`self.RotateObjectByMouse`)
        (elif (`KismetStringLibrary.EqualEqual_StrStr` (`self.NamePista`) "S_Pedant")
          (set `self.RotateObject?` true)
          (`SceneComponent.SetVisibility` (`self.Object`) true true)
          (`self.RotateObject`)))))
  (:`Released`
    (if (`self.Inspection?`)
      _
      (elif (`self.RotateObjectByMouse?`)
        (set `self.RotateObjectByMouse?` false)
        (set `self.RotateObject?` true)
        (`self.RotateObject`)))))

(event `RotateObject`
  (bind _returnvalue (* (`GameplayStatics.GetWorldDeltaSeconds`) (`self.SpeedRotate`)))
  (if (`self.RotateObject?`)
    (`KismetSystemLibrary.K2_SetTimerForNextTickDelegate` (delegate `RotateObject`))
    (`SceneComponent.K2_AddWorldRotation` (`self.Object`) (`KismetMathLibrary.MakeRotator` _returnvalue _returnvalue) false false)))

(event `RotateObjectByMouse`
  (bind (_deltax _deltay) (`PlayerController.GetInputMouseDelta` (`GameplayStatics.GetPlayerController` 0)))
  (if (`self.RotateObjectByMouse?`)
    (`KismetSystemLibrary.K2_SetTimerForNextTickDelegate` (delegate `RotateObjectByMouse`))
    (`SceneComponent.K2_AddWorldRotation` (`self.Object`) (* (`KismetMathLibrary.MakeRotator` _deltay 0.0 _deltax) -1.0) false false)))

(fn `AddScaleSpritesArray`
  (params (NewScale3D :type "Vector Structure"))
  (for _array_element (`self.SpritesPistas`)
    (`self.SetActorScale3D` _array_element NewScale3D)))

(fn `GetScaleAdd`
  (returns (ReturnValue :type "Vector Structure"))
  (bind _returnvalue (* (`self.SpeedZoomCamera`) (select `bool` (> (`self.GetInputAxisValue`) 0.0) :`false` 1.0 :`true` -1.0) (`GameplayStatics.GetWorldDeltaSeconds`) 0.1))
  (return (`KismetMathLibrary.MakeVector` (+ (.x (`SceneComponent.RelativeScale3D` (`self.S_SceneCrimen_2`))) _returnvalue) (.y (`SceneComponent.RelativeScale3D` (`self.S_SceneCrimen_2`))) (+ (.z (`SceneComponent.RelativeScale3D` (`self.S_SceneCrimen_2`))) _returnvalue))))

(fn `MouseLupaNoZoom`
  (`/Engine/EditorBlueprintResources/StandardMacros.IsValid` (`self.LupaNoZoom`)
    (:`Is Valid`
      _)
    (:`Is Not Valid`
      (bind _returnvalue (`|CreateWidget` "/Game/Miguel/Widgets/UI/PaC/WD_LupaNoZoom.WD_LupaNoZoom_C"))
      (set `self.LupaNoZoom` _returnvalue)))
  (`PlayerController.SetMouseCursorWidget` (`GameplayStatics.GetPlayerController` 0) "Default" (`self.LupaNoZoom`)))

(fn `MouseLupaZoom`
  (`/Engine/EditorBlueprintResources/StandardMacros.IsValid` (`self.LupaZoom`)
    (:`Is Valid`
      _)
    (:`Is Not Valid`
      (bind _returnvalue (`|CreateWidget` "/Game/Miguel/Widgets/UI/PaC/WD_LupaZoom.WD_LupaZoom_C"))
      (set `self.LupaZoom` _returnvalue)))
  (`PlayerController.SetMouseCursorWidget` (`GameplayStatics.GetPlayerController` 0) "Default" (`self.LupaZoom`)))

(fn `MoveHorizontalAxis`
  (params (`Move Axis` :type "Float (double-precision)") (MaxMove :type "Float (double-precision)"))
  (bind (_relativelocation_x _relativelocation_y _relativelocation_z) (`KismetMathLibrary.BreakVector` (`SceneComponent.RelativeLocation` (`self.Camera`))))
  (bind _returnvalue (+ (* (`self.SpeedMoveCamera`) (`GameplayStatics.GetWorldDeltaSeconds`) (`local.Move Axis`)) (`KismetMathLibrary.BreakVector3f` (`SceneComponent.RelativeLocation` (`self.Camera`)))))
  (if (`self.Inspection?`)
    _
    (elif (!= (`local.Move Axis`) 0.0)
      (if (select `bool` (> (`local.Move Axis`) 0.0) :`false` (< _returnvalue (* (`local.MaxMove`) (`local.Move Axis`))) :`true` (> _returnvalue (* (`local.MaxMove`) (`local.Move Axis`))))
        (`SceneComponent.K2_SetRelativeLocation` (`self.Camera`) (`KismetMathLibrary.MakeVector` (* (`local.Move Axis`) (`local.MaxMove`)) _relativelocation_y _relativelocation_z) false false)
        (else
          (`SceneComponent.K2_AddRelativeLocation` (`self.Camera`) (`KismetMathLibrary.MakeVector` (* (`self.SpeedMoveCamera`) (`GameplayStatics.GetWorldDeltaSeconds`) (`local.Move Axis`))) false false))))))

(fn `MoveVerticalAxis`
  (params (`Move Axis` :type "Float (double-precision)") (MaxMove :type "Float (double-precision)"))
  (bind (_relativelocation_x _relativelocation_y) (`KismetMathLibrary.BreakVector` (`SceneComponent.RelativeLocation` (`self.Camera`))))
  (bind _returnvalue (+ (* (`self.SpeedMoveCamera`) (`GameplayStatics.GetWorldDeltaSeconds`) (`local.Move Axis`)) (`.Z` (`KismetMathLibrary.BreakVector3f` (`SceneComponent.RelativeLocation` (`self.Camera`))))))
  (if (`self.Inspection?`)
    _
    (elif (!= (`local.Move Axis`) 0.0)
      (set `self.Move?` true)
      (if (select `bool` (> (`local.Move Axis`) 0.0) :`false` (< _returnvalue (* (`local.MaxMove`) (`local.Move Axis`))) :`true` (> _returnvalue (* (`local.MaxMove`) (`local.Move Axis`))))
        (`SceneComponent.K2_SetRelativeLocation` (`self.Camera`) (`KismetMathLibrary.MakeVector` _relativelocation_x _relativelocation_y (* (`local.Move Axis`) (`local.MaxMove`))) false false)
        (else
          (`SceneComponent.K2_AddRelativeLocation` (`self.Camera`) (`KismetMathLibrary.MakeVector` 0.0 0.0 (* (`self.SpeedMoveCamera`) (`GameplayStatics.GetWorldDeltaSeconds`) (`local.Move Axis`))) false false))))))

(fn `SetScaleSprites`
  (params (NewScale3D :type "Vector Structure"))
  (`self.AddScaleSpritesArray` NewScale3D)
  (`SceneComponent.SetRelativeScale3D` (`self.S_SceneCrimen_2`) (`local.NewScale3D`)))

(fn `UserConstructionScript`)

(fn `ZoomBySpriteNew`
  (params (AddRelativeLocation :type "Vector Structure"))
  (locals (CamZoom :type "Float (double-precision)"))
  (if (< (`self.GetInputAxisValue`) 0.0)
    (if (< (.x (`local.AddRelativeLocation`)) 2.0)
      (set `self.ZoomChange` 1.0)
      (`self.SetScaleSprites` (`local.AddRelativeLocation`) :!label _label)
      (else
        (`self.SetScaleSprites` (2.0 1.0 2.0))))
    (set `self.MaxHorizontal` (+ (`self.MaxHorizontal`) (* (`self.SpeedZoomCamera`) (`self.ZoomChange`) (`GameplayStatics.GetWorldDeltaSeconds`) 96.0)))
    (set `self.MaxVertical` (+ (`self.MaxVertical`) (* (`self.SpeedZoomCamera`) (`self.ZoomChange`) (`GameplayStatics.GetWorldDeltaSeconds`) 54.0)))
    (else
      (`SceneComponent.K2_SetRelativeLocation` (`self.Camera`) (0.0 800.0 0.0) false false)
      (if (> (`KismetMathLibrary.BreakVector3f` (`local.AddRelativeLocation`)) 1.0)
        (set `self.ZoomChange` -1.0)
        (goto _label)
        (else
          (`self.SetScaleSprites` (1.0 1.0 1.0))
          (set `self.MaxHorizontal` 0.0)
          (set `self.MaxVertical` 0.0))))))