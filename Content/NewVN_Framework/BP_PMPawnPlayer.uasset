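; Player pawn for a 2D visual novel scene, holding the background and character sprites with their lights and enabling mouse input.
; Left click asks BPTypeWrite to advance to the next scene.
; The construction script picks the background from an enum, while ChangeSpriteCharacter swaps the speaker sprite when the name changes and plays a timeline to raise or reverse the character light.
; The H key triggers a second timeline driving both character and background lights.
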(event `self.ReceiveBeginPlay`
  (bind _returnvalue (`GameplayStatics.GetPlayerController` 0))
  (set `PlayerController.bShowMouseCursor` true _returnvalue)
  (set `PlayerController.bEnableMouseOverEvents` true _returnvalue)
  (set `PlayerController.bEnableClickEvents` true _returnvalue))

(event `Key|LeftMouseButton`
  (params (Key :type "Key Structure"))
  (:`Pressed`
    (`/Engine/EditorBlueprintResources/StandardMacros.IsValid` (`self.BP_TypeWrite`)
      (:`Is Valid`
        (`/Game/NewVN_Framework/BP_TypeWrite.DisNextScene` (`self.BP_TypeWrite`))))))

(event `IncrementLight`
  (params (`Play Mode` :type "EUMGSequencePlayMode Enum" :default "Forward"))
  (switch `EUMGSequencePlayMode` `Play Mode`
    (:`Forward`
      (bind (_direction _intensity) (`Timeline|TImeIntensityLigthCharacter` :!via `PlayFromStart` :!label _label)
        (:`Update`
          (`LightComponent.SetIntensity` (`self.LightCharacter`) _intensity))))
    (:`Reverse`
      (goto _label :!via `ReverseFromEnd`))))

(event `LightTimeOff`
  (bind (_direction _intensity _backgroundlight) (`Timeline|T` :!via `PlayFromStart`)
    (:`Update`
      (`LightComponent.SetIntensity` (`self.LightCharacter`) _intensity)
      (`LightComponent.SetIntensity` (`self.BackgroundLight`) _backgroundlight))))

(event `Key|H`
  (params (Key :type "Key Structure"))
  (:`Pressed`
    (`self.LightTimeOff`)))

(fn `ChangeBackground`
  (params (Character :type "/Game/NewVN_Framework/Enums/EN_Background2D Enum" :default "NewEnumerator0"))
  (bind (_casamatthew _despacho _crimen _interrogatorio) (break `/Game/NewVN_Framework/Structures/ST_Background2D` (`self.ST_Background2D`)))
  (`PaperSpriteComponent.SetSprite` (`self.Sprite_Background`) (select `/Game/NewVN_Framework/Enums/EN_Background2D` (`local.Character`) :`NewEnumerator0` _interrogatorio :`NewEnumerator1` _crimen :`NewEnumerator2` _despacho :`NewEnumerator3` _casamatthew)))

(fn `ChangeSpriteCharacter`
  (params (NewSpriteCharacter :type "PaperSprite Object Reference") (NameCharacter :type "/Game/NewVN_Framework/Enums/EN_Characters Enum" :default "NewEnumerator4"))
  (`/Engine/EditorBlueprintResources/StandardMacros.IsValid` NewSpriteCharacter
    (:`Is Valid`
      (if (`|EnumInequality` (`self.Name Character`) NameCharacter)
        (set `self.Name Character` NameCharacter)
        (`PaperSpriteComponent.SetSprite` (`self.SpriteCharacter`) NewSpriteCharacter)
        (`self.IncrementLight` "Forward")))
    (:`Is Not Valid`
      (if (`|EnumInequality` (`self.Name Character`) NameCharacter)
        (set `self.Name Character` NameCharacter)
        (`self.IncrementLight` "Reverse")))))

(fn `UserConstructionScript`
  (`self.ChangeBackground` (`self.EN_Background2D`)))