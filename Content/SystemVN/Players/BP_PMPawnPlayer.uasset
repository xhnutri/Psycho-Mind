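; Player pawn for a visual-novel scene, presenting a background sprite and a character sprite with their lights.
; It enables mouse input and forwards clicks to the typewriter object to trigger the next scene.
; Construction picks the background from an enum, and name changes swap the character sprite or fade its light via timelines.
; Other functions toggle visibility, animate background and character lighting together, and set a pen cursor widget.
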(event `NotVisible`
  (`SceneComponent.SetVisibility` (`self.DefaultSceneRoot`) false true))

(event `InitVisble`
  (`SceneComponent.SetVisibility` (`self.DefaultSceneRoot`) true true))

(event `self.ReceiveBeginPlay`
  (bind _returnvalue (`GameplayStatics.GetPlayerController` 0))
  (set `PlayerController.bShowMouseCursor` true _returnvalue)
  (set `PlayerController.bEnableMouseOverEvents` true _returnvalue)
  (set `PlayerController.bEnableClickEvents` true _returnvalue))

(event `InputAction|Click`
  (params (Key :type "Key Structure"))
  (:`Pressed`
    (`/Engine/EditorBlueprintResources/StandardMacros.IsValid` (`self.BP_TypeWrite`)
      (:`Is Valid`
        (`/Game/SystemVN/SystemWriter/BP_TypeWrite.DisNextScene` (`self.BP_TypeWrite`))))))

(event `IncrementLight`
  (params (`Play Mode` :type "EUMGSequencePlayMode Enum" :default "Forward"))
  (switch `EUMGSequencePlayMode` `Play Mode`
    (:`Forward`
      (bind (_direction _intensity) (`Timeline|TImeIntensityLigthCharacter` :!via `PlayFromStart` :!label _label)
        (:`Update`
          (`LightComponent.SetIntensity` (`self.LightCharacter`) _intensity))))
    (:`Reverse`
      (goto _label :!via `ReverseFromEnd`))))

(event `LightTimeOffOn`
  (params (Selection :type "EUMGSequencePlayMode Enum" :default "Forward") (`IsCharacter?` :type Boolean))
  (switch `EUMGSequencePlayMode` Selection
    (:`Forward`
      (bind (_direction _intensity _backgroundlight) (`Timeline|TimerThinkin` :!via `PlayFromStart` :!label _label_2)
        (:`Update`
          (if `IsCharacter?`
            (`LightComponent.SetIntensity` (`self.LightCharacter`) _intensity))
          (`LightComponent.SetIntensity` (`self.BackgroundLight`) _backgroundlight))))
    (:`Reverse`
      (goto _label_2 :!via `ReverseFromEnd`))))

(fn `ChangeBackground`
  (params (Character :type "/Game/SystemVN/Enums/EN_Background2DNames Enum" :default "NewEnumerator0"))
  (bind (_casamatthew _despacho _crimen _interrogatorio) (break `/Game/SystemVN/Structures/ST_Background2DSprites` (`self.ST_Background2D`)))
  (`PaperSpriteComponent.SetSprite` (`self.Sprite_Background`) (select `/Game/SystemVN/Enums/EN_Background2DNames` (`self.EN_Background2D`) :`NewEnumerator0` _interrogatorio :`NewEnumerator1` _crimen :`NewEnumerator2` _despacho :`NewEnumerator3` _casamatthew)))

(fn `ChangeMouse`
  (bind _returnvalue (`|CreateWidget` "/Game/Miguel/Widgets/WD_PenClick.WD_PenClick_C"))
  (`PlayerController.SetMouseCursorWidget` (`GameplayStatics.GetPlayerController` 0) "Default" _returnvalue))

(fn `ChangeSpriteCharacter`
  (params (NewSpriteCharacter :type "PaperSprite Object Reference") (NameCharacter :type "/Game/SystemVN/Enums/EN_Characters Enum" :default "NewEnumerator4"))
  (`/Engine/EditorBlueprintResources/StandardMacros.IsValid` NewSpriteCharacter
    (:`Is Valid`
      (if (`|EnumInequality` (`self.Name Character`) NameCharacter)
        (set `self.Name Character` NameCharacter)
        (`PaperSpriteComponent.SetSprite` (`self.SpriteCharacter`) NewSpriteCharacter)
        (`self.IncrementLight` "Forward")))
    (:`Is Not Valid`
      (if (`|EnumInequality` (`self.Name Character`) NameCharacter)
        (set `self.Name Character` NameCharacter)
        (`self.IncrementLight` "Reverse")))))

(fn `UserConstructionScript`
  (`self.ChangeBackground` (`self.EN_Background2D`)))