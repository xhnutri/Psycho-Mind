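; Point-and-click player for a crime-scene investigation where the cursor hovers and clicks Paper2D clue sprites.
; Tick traces under the mouse to swap the scene sprite and magnifier cursor, and edge-pans the camera within zoom-dependent limits.
; Zoom scales the sprites rather than moving the lens.
; Clicking a clue records it, matches its name to a scene enum for BPTypeWrite, and can reveal a rotating, mouse-draggable object.
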(event `self.ReceiveBeginPlay`
  (bind _returnvalue (`GameplayStatics.GetPlayerController` 0))
  (`self.MouseLupaNoZoom`)
  (set `self.InitSprite` (`PaperSpriteComponent.GetSprite` (`self.S_SceneCrimen_2`)))
  (set `PlayerController.bShowMouseCursor` true _returnvalue)
  (set `PlayerController.bEnableMouseOverEvents` true _returnvalue)
  (set `PlayerController.bEnableClickEvents` true _returnvalue))

(event `self.ReceiveTick`
  (params (DeltaSeconds :type "Float (single-precision)"))
  (bind (_worldlocation _worlddirection) (`PlayerController.DeprojectMousePositionToWorld` (`GameplayStatics.GetPlayerController` 0)))
  (`|ExecutionSequence`
    (:`then_0`
      (if (not (`self.InitScene?`))
        (bind (_outhit _returnvalue) (`KismetSystemLibrary.LineTraceSingle` :`Start` _worldlocation :`End` (+ _worldlocation (* _worlddirection 10000)) :`TraceChannel` "TraceTypeQuery1" :`bIgnoreSelf` false))
        (if _returnvalue
          (bind _aspaper_sprite_component (cast `PaperSpriteComponent` (`.HitComponent` (`GameplayStatics.BreakHitResult` _outhit)))
            (:`then`
              (bind _returnvalue_2 (`PaperSpriteComponent.GetSprite` _aspaper_sprite_component))
              (`PaperSpriteComponent.SetSprite` (`self.S_SceneCrimen_2`) _returnvalue_2)
              (set `self.NamePista` (`KismetSystemLibrary.GetObjectName` _returnvalue_2))
              (if (not (`self.ViewObject?`))
                (set `self.ViewObject?` true)
                (`self.MouseLupaZoom`)))
            (:`CastFailed`
              (set `self.NamePista` "" :!label _label)
              (`PaperSpriteComponent.SetSprite` (`self.S_SceneCrimen_2`) (`self.InitSprite`))
              (if (`self.ViewObject?`)
                (set `self.ViewObject?` false)
                (`self.MouseLupaNoZoom`))))
          (else
            (goto _label)))))
    (:`then_1`
      (if (not (`self.InitScene?`))
        (`self.CreateMouseMove`)))))

(event `InitVisibleScene`
  (`SceneComponent.SetVisibility` (`self.RectLight`) true false)
  (`SceneComponent.SetVisibility` (`self.S_SceneCrimen_2`) true false))

(event `InputAxis|ZoomObject`
  (params (AxisValue :type "Float (single-precision)"))
  (`self.ZoomBySpriteNew` (`self.GetScaleAdd`)))

(event `InputAction|Click`
  (params (Key :type "Key Structure"))
  (:`Pressed`
    (if (`self.InitScene?`)
      (`/Engine/EditorBlueprintResources/StandardMacros.IsValid` (`self.BP_TypeWrite`)
        (:`Is Valid`
          (`/Game/SystemVN/SystemWriter/BP_TypeWrite.DisNextScene` (`self.BP_TypeWrite`))))
      (else
        (bind _enumvalue (foreach `/Game/SystemVN/Enums/EN_ScenesNames` false)
          (:`LoopBody`
            (if (`KismetStringLibrary.EqualEqual_StrStr` (`|GetEnumeratorNameAsString` _enumvalue) (`KismetStringLibrary.Concat_StrStr` "Pista" (`self.NamePista`)))
              (`self.SaveObjects` (`self.NamePista`))
              (set `self.InitScene?` true)
              (`SceneComponent.K2_SetRelativeLocation` (`self.Camera`) (0.0 800.0 0.0) false false)
              (set `self.RotateObject?` true)
              (if (`|EnumEquality` _enumvalue "NewEnumerator26")
                (`SceneComponent.SetVisibility` (`self.Object`) true true)
                (`self.RotateObject`))
              (`/Game/SystemVN/SystemWriter/BP_TypeWrite.InitScene` (`self.BP_TypeWrite`) (`KismetStringLibrary.Conv_StringToName` (`KismetStringLibrary.Concat_StrStr` "Pista" (`self.NamePista`)))))))))))

(event `RotateObject`
  (bind _returnvalue (* (`GameplayStatics.GetWorldDeltaSeconds`) (`self.SpeedRotate`)))
  (if (`self.RotateObject?`)
    (`KismetSystemLibrary.K2_SetTimerForNextTickDelegate` (delegate `RotateObject`))
    (`SceneComponent.K2_AddWorldRotation` (`self.Object`) (`KismetMathLibrary.MakeRotator` _returnvalue _returnvalue) false false)))

(event `RotateObjectByMouse`
  (bind (_deltax _deltay) (`PlayerController.GetInputMouseDelta` (`GameplayStatics.GetPlayerController` 0)))
  (if (`self.RotateObjectByMouse?`)
    (`KismetSystemLibrary.K2_SetTimerForNextTickDelegate` (delegate `RotateObjectByMouse`))
    (`SceneComponent.K2_AddWorldRotation` (`self.Object`) (* (`KismetMathLibrary.MakeRotator` _deltay 0.0 _deltax) -1.0) false false)))

(event `Key|RightMouseButton`
  (params (Key :type "Key Structure"))
  (:`Pressed`
    (if (`self.RotateObject?`)
      (set `self.RotateObject?` false)
      (set `self.RotateObjectByMouse?` true)
      (`self.RotateObjectByMouse`)))
  (:`Released`
    (if (`self.RotateObjectByMouse?`)
      (set `self.RotateObjectByMouse?` false)
      (set `self.RotateObject?` true)
      (`self.RotateObject`))))

(fn `AddScaleSpritesArray`
  (params (NewScale3D :type "Vector Structure"))
  (`SceneComponent.SetRelativeScale3D` (`self.Pistas`) NewScale3D)
  (`SceneComponent.SetRelativeScale3D` (`self.PistasCut`) NewScale3D))

(fn `CreateMouseMove`
  (bind (_returnvalue_x _returnvalue_y) (`KismetMathLibrary.BreakVector2D` (`WidgetLayoutLibrary.GetViewportSize`)))
  (bind (_worldlocation _worlddirection _returnvalue) (`PlayerController.DeprojectMousePositionToWorld` (`GameplayStatics.GetPlayerController` 0)))
  (bind _x (.x _worlddirection))
  (bind _z (.z _worlddirection))
  (if _returnvalue
    (`self.SetVariablesMoveMouse` (.x (`KismetMathLibrary.Vector_GetAbs` _worldlocation)) (`KismetMathLibrary.Abs` _x) (.x (`.WorldDirection` (`PlayerController.DeprojectScreenPositionToWorld` (`GameplayStatics.GetPlayerController` 0) _returnvalue_x _returnvalue_y))) (`self.MaxHorizontal`) (`KismetMathLibrary.SelectFloat` 1.0 -1.0 (> _x 0.0)))
    (`self.SetVariablesMoveMouse` (.z (`KismetMathLibrary.Vector_GetAbs` _worldlocation)) (`KismetMathLibrary.Abs` _z) (.z (`.WorldDirection` (`PlayerController.DeprojectScreenPositionToWorld` (`GameplayStatics.GetPlayerController` 0) _returnvalue_x _returnvalue_y))) (`self.MaxVertical`) (`KismetMathLibrary.SelectFloat` 1.0 -1.0 (> _z 0.0)) true)))

(fn `GetScaleAdd`
  (returns (ReturnValue :type "Vector Structure"))
  (bind _returnvalue (* (`self.SpeedZoomCamera`) (select `bool` (> (`self.GetInputAxisValue`) 0.0) :`false` 1.0 :`true` -1.0) (`GameplayStatics.GetWorldDeltaSeconds`) 0.1))
  (return (`KismetMathLibrary.MakeVector` (+ (.x (`SceneComponent.RelativeScale3D` (`self.S_SceneCrimen_2`))) _returnvalue) (.y (`SceneComponent.RelativeScale3D` (`self.S_SceneCrimen_2`))) (+ (.z (`SceneComponent.RelativeScale3D` (`self.S_SceneCrimen_2`))) _returnvalue))))

(fn `MouseLupaNoZoom`
  (`/Engine/EditorBlueprintResources/StandardMacros.IsValid` (`self.LupaNoZoom`)
    (:`Is Valid`
      _)
    (:`Is Not Valid`
      (bind _returnvalue (`|CreateWidget` "/Game/Miguel/Widgets/UI/PaC/WD_LupaNoZoom.WD_LupaNoZoom_C"))
      (set `self.LupaNoZoom` _returnvalue)))
  (`PlayerController.SetMouseCursorWidget` (`GameplayStatics.GetPlayerController` 0) "Default" (`self.LupaNoZoom`)))

(fn `MouseLupaZoom`
  (`/Engine/EditorBlueprintResources/StandardMacros.IsValid` (`self.LupaZoom`)
    (:`Is Valid`
      _)
    (:`Is Not Valid`
      (bind _returnvalue (`|CreateWidget` "/Game/Miguel/Widgets/UI/PaC/WD_LupaZoom.WD_LupaZoom_C"))
      (set `self.LupaZoom` _returnvalue)))
  (`PlayerController.SetMouseCursorWidget` (`GameplayStatics.GetPlayerController` 0) "Default" (`self.LupaZoom`)))

(fn `MoveHorizontalAxis`
  (params (`Move Axis` :type "Float (double-precision)") (MaxMove :type "Float (double-precision)"))
  (bind (_relativelocation_x _relativelocation_y _relativelocation_z) (`KismetMathLibrary.BreakVector` (`SceneComponent.RelativeLocation` (`self.Camera`))))
  (bind _returnvalue (+ (* (`self.SpeedMoveCamera`) (`GameplayStatics.GetWorldDeltaSeconds`) (`local.Move Axis`)) (`KismetMathLibrary.BreakVector3f` (`SceneComponent.RelativeLocation` (`self.Camera`)))))
  (if (`self.Inspection?`)
    _
    (elif (!= (`local.Move Axis`) 0.0)
      (if (select `bool` (> (`local.Move Axis`) 0.0) :`false` (< _returnvalue (* (`local.MaxMove`) (`local.Move Axis`))) :`true` (> _returnvalue (* (`local.MaxMove`) (`local.Move Axis`))))
        (`SceneComponent.K2_SetRelativeLocation` (`self.Camera`) (`KismetMathLibrary.MakeVector` (* (`local.Move Axis`) (`local.MaxMove`)) _relativelocation_y _relativelocation_z) false false)
        (else
          (`SceneComponent.K2_AddRelativeLocation` (`self.Camera`) (`KismetMathLibrary.MakeVector` (* (`self.SpeedMoveCamera`) (`GameplayStatics.GetWorldDeltaSeconds`) (`local.Move Axis`))) false false))))))

(fn `MoveVerticalAxis`
  (params (`Move Axis` :type "Float (double-precision)") (MaxMove :type "Float (double-precision)"))
  (bind (_relativelocation_x _relativelocation_y) (`KismetMathLibrary.BreakVector` (`SceneComponent.RelativeLocation` (`self.Camera`))))
  (bind _returnvalue (+ (* (`self.SpeedMoveCamera`) (`GameplayStatics.GetWorldDeltaSeconds`) (`local.Move Axis`)) (`.Z` (`KismetMathLibrary.BreakVector3f` (`SceneComponent.RelativeLocation` (`self.Camera`))))))
  (if (`self.Inspection?`)
    _
    (elif (!= (`local.Move Axis`) 0.0)
      (set `self.Move?` true)
      (if (select `bool` (> (`local.Move Axis`) 0.0) :`false` (< _returnvalue (* (`local.MaxMove`) (`local.Move Axis`))) :`true` (> _returnvalue (* (`local.MaxMove`) (`local.Move Axis`))))
        (`SceneComponent.K2_SetRelativeLocation` (`self.Camera`) (`KismetMathLibrary.MakeVector` _relativelocation_x _relativelocation_y (* (`local.Move Axis`) (`local.MaxMove`))) false false)
        (else
          (`SceneComponent.K2_AddRelativeLocation` (`self.Camera`) (`KismetMathLibrary.MakeVector` 0.0 0.0 (* (`self.SpeedMoveCamera`) (`GameplayStatics.GetWorldDeltaSeconds`) (`local.Move Axis`))) false false))))))

(fn `SaveObjects`
  (params (PistaName :type String))
  (locals (ExitsName :type Boolean))
  (bind _returnvalue (`self.GetComponentsByTag` "/Script/Paper2D.PaperSpriteComponent" (`KismetStringLibrary.Conv_StringToName` (`local.PistaName`))))
  (bind _returnvalue_2 (`self.GetComponentsByTag` "/Script/Paper2D.PaperSpriteComponent" (`KismetStringLibrary.Conv_StringToName` (`local.PistaName`))))
  (if (`KismetStringLibrary.NotEqual_StrStr` PistaName "S_Body")
    (if (== (`self.PistasEncontradas`) 0)
      (`KismetArrayLibrary.Array_Add` (`self.SaveNamesPistas`) (`local.PistaName`))
      (`/Engine/EditorBlueprintResources/StandardMacros.IncrementInt` (`self.PistasEncontradas`)
        (:`  `
          (if (> (`KismetArrayLibrary.Array_Length` _returnvalue) 0)
            (`SceneComponent.SetVisibility` (`|GetArrayItem` _returnvalue) true false))))
      (else
        (for _array_element (`self.SaveNamesPistas`)
          (if (`KismetStringLibrary.EqualEqual_StrStr` _array_element (`local.PistaName`))
            (set `local.ExitsName` true)
            (break)))
        (if (not (`local.ExitsName`))
          (`KismetArrayLibrary.Array_Add` (`self.SaveNamesPistas`) (`local.PistaName`))
          (`/Engine/EditorBlueprintResources/StandardMacros.IncrementInt` (`self.PistasEncontradas`)
            (:`  `
              (if (> (`KismetArrayLibrary.Array_Length` _returnvalue_2) 0)
                (`SceneComponent.SetVisibility` (`|GetArrayItem` _returnvalue_2) true false)))))))))

(fn `SetScaleSprites`
  (params (NewScale3D :type "Vector Structure"))
  (`self.AddScaleSpritesArray` NewScale3D)
  (`SceneComponent.SetRelativeScale3D` (`self.S_SceneCrimen_2`) (`local.NewScale3D`)))

(fn `SetVariablesMoveMouse`
  (params (MouseLocation :type "Float (double-precision)") (MouseDirection :type "Float (double-precision)") (ScreenDirection :type "Float (double-precision)") (MaxLocation :type "Float (double-precision)") (SetDirection :type "Float (double-precision)") (IsVertical :type Boolean))
  (locals (Direction :type "Float (double-precision)"))
  (bind _returnvalue (* (`local.MaxLocation`) (`local.SetDirection`)))
  (bind _returnvalue_2 (* (`self.SpeedMoveCamera`) (`GameplayStatics.GetWorldDeltaSeconds`) (`local.SetDirection`)))
  (bind (_relativelocation_x _relativelocation_y _relativelocation_z) (`KismetMathLibrary.BreakVector` (`SceneComponent.RelativeLocation` (`self.Camera`))))
  (bind (_relativelocation_x_2 _relativelocation_y_2) (`KismetMathLibrary.BreakVector` (`SceneComponent.RelativeLocation` (`self.Camera`))))
  (if (> (`local.MouseDirection`) (* (`KismetMathLibrary.Abs` (`local.ScreenDirection`)) (/ 7.0 8.0)))
    (if (> (`local.MouseLocation`) (`local.MaxLocation`))
      (`SceneComponent.K2_SetRelativeLocation` (`self.Camera`) (select `bool` (`local.IsVertical`) :`false` (`KismetMathLibrary.MakeVector` _returnvalue _relativelocation_y _relativelocation_z) :`true` (`KismetMathLibrary.MakeVector` _relativelocation_x_2 _relativelocation_y_2 _returnvalue)) false false)
      (else
        (`SceneComponent.K2_AddRelativeLocation` (`self.Camera`) (select `bool` (`local.IsVertical`) :`false` (`KismetMathLibrary.MakeVector` _returnvalue_2) :`true` (`KismetMathLibrary.MakeVector` 0.0 0.0 _returnvalue_2)) false false)))))

(fn `UserConstructionScript`)

(fn `ZoomBySpriteNew`
  (params (AddRelativeLocation :type "Vector Structure"))
  (locals (CamZoom :type "Float (double-precision)") (ScaleAdd :type "Vector Structure"))
  (if (`self.InitScene?`)
    _
    (elif (!= (`self.GetInputAxisValue`) 0.0)
      (set `local.ScaleAdd` (`self.GetScaleAdd`))
      (if (< (`self.GetInputAxisValue`) 0.0)
        (if (< (.x (`local.ScaleAdd`)) 2.0)
          (set `self.ZoomChange` 1.0)
          (`self.SetScaleSprites` (`local.ScaleAdd`) :!label _label)
          (set `self.MaxHorizontal` (+ (`self.MaxHorizontal`) (* (`self.SpeedZoomCamera`) (`self.ZoomChange`) (`GameplayStatics.GetWorldDeltaSeconds`) 96.0)))
          (set `self.MaxVertical` (+ (`self.MaxVertical`) (* (`self.SpeedZoomCamera`) (`self.ZoomChange`) (`GameplayStatics.GetWorldDeltaSeconds`) 54.0)))
          (else
            (`self.SetScaleSprites` (2.0 1.0 2.0))
            (set `self.MaxHorizontal` 960.0)
            (set `self.MaxVertical` 540.0)))
        (else
          (`SceneComponent.K2_SetRelativeLocation` (`self.Camera`) (0.0 800.0 0.0) false false)
          (if (> (`KismetMathLibrary.BreakVector3f` (`local.ScaleAdd`)) 1.0)
            (set `self.ZoomChange` -1.0)
            (goto _label)
            (else
              (`self.SetScaleSprites` (1.0 1.0 1.0))
              (set `self.MaxHorizontal` 0.0)
              (set `self.MaxVertical` 0.0))))))))